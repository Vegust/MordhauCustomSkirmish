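; Game state for a Mordhau custom skirmish mode, holding configurable round rules, team names and scores.
; ApplySettings copies values into the round variables; the server loads them from a startup save, and clients mirror some on BeginPlay.
; When a team reaches the round target, the server logs the match to a capped save-game history, if enabled, and ends it through the game mode.
; Admin-style events pause, reset scores, end rounds and skip warmup.
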(event Custom|ApplySettings
  (params (Regen :type Boolean) (End :type Integer) (Start :type Integer) (Round :type Integer) (Warmup :type Integer) (MinP :type Integer) (RtW :type Integer) (Late :type Integer) (BlueName :type String) (RedName :type String) (SaveMatch :type Boolean) (IRLDeath :type Boolean) (Scoring :type Boolean))
  (Utilities|FlowControl|Sequence
    (:then_0
      (Variables|Default|SetbAllowHealthRegen Regen))
    (:then_1
      (bind _output_get (Variables|SettingsSkirmish|SetEndDur End))
      (Variables|Default|SetRoundEndDuration (Math|Conversions|ToFloat(Integer) _output_get)))
    (:then_2
      (bind _output_get_2 (Variables|SettingsSkirmish|SetStartDur Start))
      (Variables|Default|SetRoundStartDuration (Math|Conversions|ToFloat(Integer) _output_get_2)))
    (:then_3
      (bind _output_get_3 (Variables|SettingsSkirmish|SetRoundDur Round))
      (Variables|Default|SetRoundDuration (Math|Conversions|ToFloat(Integer) _output_get_3)))
    (:then_4
      (bind _output_get_4 (Variables|SettingsSkirmish|SetWarmupDur Warmup))
      (Variables|Default|SetDefaultWarmupTime (Math|Conversions|ToFloat(Integer) _output_get_4)))
    (:then_5
      (bind _output_get_5 (Variables|SettingsSkirmish|SetMinPl MinP))
      (Variables|Default|SetMinPlayersToStart _output_get_5))
    (:then_6
      (bind _output_get_6 (Variables|SettingsSkirmish|SetRoundsToWin RtW))
      (Variables|Default|SetWinConditionRounds _output_get_6))
    (:then_7
      (bind _output_get_7 (Variables|SettingsSkirmish|SetLateDur Late))
      (Variables|Default|SetLateRoundSpawnDuration (Math|Conversions|ToFloat(Integer) _output_get_7)))
    (:then_8
      (Utilities|Array|SetArrayElem (Variables|Default|GetTeamNames) 0 RedName)
      (Utilities|Array|SetArrayElem (Variables|Default|GetTeamNames) 1 BlueName)
      (Variables|Default|SetTeamNames (Variables|Default|GetTeamNames)))
    (:then_9
      (Variables|SettingsSkirmish|SetSaveMatch SaveMatch))
    (:then_10
      (Variables|SettingsSkirmish|SetIRLDeath IRLDeath))
    (:then_11
      (bind _asbp_custom_skirmish_game_mode (Utilities|Casting|CastToBP_CustomSkirmishGameMode (Game|GetGameMode)))
      (Variables|/Script/Mordhau.MordhauGameMode|SetbIsScoringDisabled _asbp_custom_skirmish_game_mode (not Scoring)))))

(event Custom|ApplyTeamScores
  (params (Red :type Integer) (Blue :type Integer))
  (bind _teamscores (Variables|Default|GetTeamScores))
  (Utilities|FlowControl|Sequence
    (:then_0
      (Utilities|Array|SetArrayElem _teamscores 0 (Math|Conversions|ToFloat(Integer) Red)))
    (:then_1
      (Utilities|Array|SetArrayElem _teamscores 1 (Math|Conversions|ToFloat(Integer) Blue)))))

(event Custom|ServerResetScores
  (for _array_element (Variables|Default|GetPlayerArray)
    (bind _asbp_mordhau_player_state (Utilities|Casting|CastToBP_MordhauPlayerState _array_element))
    (Class|MordhauPlayerState|AddScore _asbp_mordhau_player_state (Math|Float|Round (* (Variables|/Script/Engine.PlayerState|GetScore _asbp_mordhau_player_state) -1.0)))
    (Variables|/Script/Mordhau.MordhauPlayerState|SetAssists _asbp_mordhau_player_state 0)
    (Variables|/Script/Mordhau.MordhauPlayerState|SetKills _asbp_mordhau_player_state 0)
    (Variables|/Script/Mordhau.MordhauPlayerState|SetDeaths _asbp_mordhau_player_state 0)))

(event Custom|SaveStartupSettings
  (bind _startupsave (Variables|Default|GetStartupSave))
  (bind _teamnames (Variables|Default|GetTeamNames))
  (Variables|/Game/Mordhau/Maps/CustomSkirmish/Saves/SkirmishSettingsSave.SkirmishSettingsSave_C|SetRegen _startupsave (Variables|Default|GetbAllowHealthRegen))
  (Variables|/Game/Mordhau/Maps/CustomSkirmish/Saves/SkirmishSettingsSave.SkirmishSettingsSave_C|SetEndDur _startupsave (Variables|SettingsSkirmish|GetEndDur))
  (Variables|/Game/Mordhau/Maps/CustomSkirmish/Saves/SkirmishSettingsSave.SkirmishSettingsSave_C|SetStartDur _startupsave (Variables|SettingsSkirmish|GetStartDur))
  (Variables|/Game/Mordhau/Maps/CustomSkirmish/Saves/SkirmishSettingsSave.SkirmishSettingsSave_C|SetRoundsToWin _startupsave (Variables|SettingsSkirmish|GetRoundsToWin))
  (Variables|/Game/Mordhau/Maps/CustomSkirmish/Saves/SkirmishSettingsSave.SkirmishSettingsSave_C|SetWarmupDur _startupsave (Variables|SettingsSkirmish|GetWarmupDur))
  (Variables|/Game/Mordhau/Maps/CustomSkirmish/Saves/SkirmishSettingsSave.SkirmishSettingsSave_C|SetLateDur _startupsave (Variables|SettingsSkirmish|GetLateDur))
  (Variables|/Game/Mordhau/Maps/CustomSkirmish/Saves/SkirmishSettingsSave.SkirmishSettingsSave_C|SetMinPl _startupsave (Variables|SettingsSkirmish|GetMinPl))
  (Variables|/Game/Mordhau/Maps/CustomSkirmish/Saves/SkirmishSettingsSave.SkirmishSettingsSave_C|SetSaveToHistory _startupsave (Variables|SettingsSkirmish|GetSaveMatch))
  (Variables|/Game/Mordhau/Maps/CustomSkirmish/Saves/SkirmishSettingsSave.SkirmishSettingsSave_C|SetBlueName _startupsave (Utilities|Array|Get(acopy) _teamnames 1))
  (Variables|/Game/Mordhau/Maps/CustomSkirmish/Saves/SkirmishSettingsSave.SkirmishSettingsSave_C|SetRealisticDeath _startupsave (Variables|SettingsSkirmish|GetIRLDeath))
  (Variables|/Game/Mordhau/Maps/CustomSkirmish/Saves/SkirmishSettingsSave.SkirmishSettingsSave_C|SetRoundDur _startupsave (Variables|SettingsSkirmish|GetRoundDur))
  (Variables|/Game/Mordhau/Maps/CustomSkirmish/Saves/SkirmishSettingsSave.SkirmishSettingsSave_C|SetRedName _startupsave (Utilities|Array|Get(acopy) _teamnames))
  (SaveGame|SaveGametoSlot _startupsave (Utilities|String|MakeLiteralString "CustomSkirmish/StartupConfig")))

(event Custom|LoadStartupSettings
  (bind _returnvalue (Utilities|String|MakeLiteralString "CustomSkirmish/StartupConfig"))
  (bind _returnvalue_2 (SaveGame|DoesSaveGameExist _returnvalue))
  (if _returnvalue_2
    (bind _returnvalue_3 (SaveGame|LoadGamefromSlot _returnvalue))
    (bind _asskirmish_settings_save (Utilities|Casting|CastToSkirmishSettingsSave _returnvalue_3))
    (bind _output_get (Variables|Default|SetStartupSave _asskirmish_settings_save))
    (CallFunction|ApplySettings (Variables|/Game/Mordhau/Maps/CustomSkirmish/Saves/SkirmishSettingsSave.SkirmishSettingsSave_C|GetRegen _output_get) (Variables|/Game/Mordhau/Maps/CustomSkirmish/Saves/SkirmishSettingsSave.SkirmishSettingsSave_C|GetEndDur _output_get) (Variables|/Game/Mordhau/Maps/CustomSkirmish/Saves/SkirmishSettingsSave.SkirmishSettingsSave_C|GetStartDur _output_get) (Variables|/Game/Mordhau/Maps/CustomSkirmish/Saves/SkirmishSettingsSave.SkirmishSettingsSave_C|GetRoundDur _output_get) (Variables|/Game/Mordhau/Maps/CustomSkirmish/Saves/SkirmishSettingsSave.SkirmishSettingsSave_C|GetWarmupDur _output_get) (Variables|/Game/Mordhau/Maps/CustomSkirmish/Saves/SkirmishSettingsSave.SkirmishSettingsSave_C|GetMinPl _output_get) (Variables|/Game/Mordhau/Maps/CustomSkirmish/Saves/SkirmishSettingsSave.SkirmishSettingsSave_C|GetRoundsToWin _output_get) (Variables|/Game/Mordhau/Maps/CustomSkirmish/Saves/SkirmishSettingsSave.SkirmishSettingsSave_C|GetLateDur _output_get) (Variables|/Game/Mordhau/Maps/CustomSkirmish/Saves/SkirmishSettingsSave.SkirmishSettingsSave_C|GetBlueName _output_get) (Variables|/Game/Mordhau/Maps/CustomSkirmish/Saves/SkirmishSettingsSave.SkirmishSettingsSave_C|GetRedName _output_get) (Variables|/Game/Mordhau/Maps/CustomSkirmish/Saves/SkirmishSettingsSave.SkirmishSettingsSave_C|GetSaveToHistory _output_get) (Variables|/Game/Mordhau/Maps/CustomSkirmish/Saves/SkirmishSettingsSave.SkirmishSettingsSave_C|GetRealisticDeath _output_get) false)
    (else
      (bind _returnvalue_4 (SaveGame|CreateSaveGameObject "/Game/Mordhau/Maps/CustomSkirmish/Saves/SkirmishSettingsSave.SkirmishSettingsSave_C"))
      (Variables|Default|SetStartupSave _returnvalue_4))))

(event Custom|ServerEndRound
  (params (Winner :type Byte))
  (bind _returnvalue (Math|Conversions|ToInteger(Byte) Winner))
  (bind _teamscores (Variables|Default|GetTeamScores))
  (Variables|Default|SetWarmupEnd 0.0)
  (if (== Winner 255)
    _
    (else
      (Utilities|Array|SetArrayElem _teamscores _returnvalue (+ (Utilities|Array|Get(acopy) _teamscores _returnvalue) 1.0))))
  (Variables|Default|SetRoundInfo (Utilities|Struct|MakeSTRUCT_SkirmishRoundInfo "NewEnumerator3" Winner (GameState|GetServerWorldTimeSeconds)))
  (Variables|Default|SetbAllowSpawning false))

(event Custom|ServerSkipWarmup
  (bind _asbp_custom_skirmish_game_mode (Utilities|Casting|CastToBP_CustomSkirmishGameMode (Game|GetGameMode)))
  (Variables|Default|SetWarmupEnd 0.0)
  (Default|StartRoundStart _asbp_custom_skirmish_game_mode))

(event Custom|LoadMatchHistory
  (bind _returnvalue (Utilities|String|MakeLiteralString "CustomSkirmish/MatchHistory"))
  (bind _returnvalue_2 (SaveGame|DoesSaveGameExist _returnvalue))
  (if _returnvalue_2
    (bind _returnvalue_3 (SaveGame|LoadGamefromSlot _returnvalue))
    (bind _asmatch_history_save (Utilities|Casting|CastToMatchHistorySave _returnvalue_3))
    (bind _output_get (Variables|Default|SetMatchHistory _asmatch_history_save))
    (Variables|Default|SetMatchesLog (Variables|/Game/Mordhau/Maps/CustomSkirmish/Saves/MatchHistorySave.MatchHistorySave_C|GetMatches _output_get))
    (else
      (bind _returnvalue_4 (SaveGame|CreateSaveGameObject "/Game/Mordhau/Maps/CustomSkirmish/Saves/MatchHistorySave.MatchHistorySave_C"))
      (bind _output_get_2 (Variables|Default|SetMatchHistory _returnvalue_4))
      (Variables|Default|SetMatchesLog (Variables|/Game/Mordhau/Maps/CustomSkirmish/Saves/MatchHistorySave.MatchHistorySave_C|GetMatches _output_get_2)))))

(event Custom|LogMatch
  (bind _teamnames (Variables|Default|GetTeamNames))
  (bind _teamscores (Variables|Default|GetTeamScores))
  (bind _matchhistory (Variables|Default|GetMatchHistory))
  (bind _matches (Variables|/Game/Mordhau/Maps/CustomSkirmish/Saves/MatchHistorySave.MatchHistorySave_C|GetMatches _matchhistory))
  (if (Variables|SettingsSkirmish|GetSaveMatch)
    (bind (_redplayers _blueplayers) (CallFunction|GetTeamPlayers))
    (bind _returnvalue (Game|GetCurrentLevelName true))
    (if (Utilities|Array|IsValidIndex _matches 9)
      (Utilities|Array|RemoveIndex _matches))
    (Utilities|Array|Add _matches (Utilities|Struct|MakeMatchInfo (Utilities|Array|Get(acopy) _teamnames) (Utilities|Array|Get(acopy) _teamnames 1) _redplayers _blueplayers (Math|Float|Round (Utilities|Array|Get(acopy) _teamscores)) (Math|Float|Round (Utilities|Array|Get(acopy) _teamscores 1)) (Math|DateTime|Now) _returnvalue))
    (SaveGame|SaveGametoSlot _matchhistory (Utilities|String|MakeLiteralString "CustomSkirmish/MatchHistory"))))

(event Custom|ServerTogglePause
  (params (NewPause :type Boolean))
  (bind _asbp_custom_skirmish_player_controller (Utilities|Casting|CastToBP_CustomSkirmishPlayerController (Game|GetPlayerController 0)))
  (Default|ToggleWidgetPause _asbp_custom_skirmish_player_controller NewPause))

(event EventBeginPlay
  (|CallParentFunction)
  (Networking|SwitchHasAuthority
    (:Authority
      (CallFunction|GetCurrentSettings)
      (CallFunction|LoadStartupSettings)
      (CallFunction|LoadMatchHistory))
    (:Remote
      (Utilities|FlowControl|Sequence
        (:then_0
          (Variables|Default|SetRoundEndDuration (Math|Conversions|ToFloat(Integer) (Variables|SettingsSkirmish|GetEndDur))))
        (:then_1
          (Variables|Default|SetRoundStartDuration (Math|Conversions|ToFloat(Integer) (Variables|SettingsSkirmish|GetStartDur))))
        (:then_2
          (Variables|Default|SetRoundDuration (Math|Conversions|ToFloat(Integer) (Variables|SettingsSkirmish|GetRoundDur))))
        (:then_3
          (Variables|Default|SetWinConditionRounds (Variables|SettingsSkirmish|GetRoundsToWin)))
        (:then_4
          (Variables|Default|SetLateRoundSpawnDuration (Math|Conversions|ToFloat(Integer) (Variables|SettingsSkirmish|GetLateDur))))))))

(event EventTick
  (params (DeltaSeconds :type Float%20%28single-precision%29))
  (bind _teamscores (Variables|Default|GetTeamScores))
  (bind _roundstowin (Variables|SettingsSkirmish|GetRoundsToWin))
  (bind _returnvalue (Math|Conversions|ToFloat(Integer) _roundstowin))
  (bind _output (Utilities|Array|Get(acopy) _teamscores 1))
  (bind _returnvalue_2 (>= _output _returnvalue))
  (|CallParentFunction DeltaSeconds)
  (if (or (>= (Utilities|Array|Get(acopy) _teamscores) _returnvalue) _returnvalue_2)
    (Utilities|FlowControl|DoOnce false
      (:Completed
        (Networking|SwitchHasAuthority
          (:Authority
            (CallFunction|ServerSkipWarmup)
            (CallFunction|LogMatch)
            (Variables|Default|SetMatchEndInfo (Utilities|Struct|MakeSTRUCT_MatchEndInfo 0 (select _returnvalue_2 1 0) _returnvalue))
            (bind _asbp_custom_skirmish_game_mode (Utilities|Casting|CastToBP_CustomSkirmishGameMode (Game|GetGameMode)))
            (Variables|/Game/Mordhau/Maps/CustomSkirmish/GameModeBlueprints/BP_CustomSkirmishGameMode.BP_CustomSkirmishGameMode_C|SetEndMatch _asbp_custom_skirmish_game_mode true)
            (Class|GameMode|EndMatch _asbp_custom_skirmish_game_mode)))))))

(fn ConstructionScript
  (|CallParentFunction))

(fn GetCurrentSettings
  (Utilities|FlowControl|Sequence
    (:then_0
      (Variables|SettingsSkirmish|SetEndDur (Math|Float|Round (Variables|Default|GetRoundEndDuration))))
    (:then_1
      (Variables|SettingsSkirmish|SetStartDur (Math|Float|Round (Variables|Default|GetRoundStartDuration))))
    (:then_2
      (Variables|SettingsSkirmish|SetRoundDur (Math|Float|Round (Variables|Default|GetRoundDuration))))
    (:then_3
      (Variables|SettingsSkirmish|SetWarmupDur (Math|Float|Round (Variables|Default|GetDefaultWarmupTime))))
    (:then_4
      (Variables|SettingsSkirmish|SetMinPl (Variables|Default|GetMinPlayersToStart)))
    (:then_5
      (Variables|SettingsSkirmish|SetRoundsToWin (Variables|Default|GetWinConditionRounds)))
    (:then_6
      (Variables|SettingsSkirmish|SetLateDur (Math|Float|Round (Variables|Default|GetLateRoundSpawnDuration))))))

(fn GetTeamPlayers
  (for _array_element (Variables|Default|GetPlayerArray)
    (bind _asbp_mordhau_player_state (Utilities|Casting|CastToBP_MordhauPlayerState _array_element))
    (if (== (Variables|/Script/Mordhau.MordhauPlayerState|GetTeam _asbp_mordhau_player_state) 0)
      (Utilities|Array|Add (LocalVariables|GetRed) (Utilities|Struct|MakePlayerInfo (PlayerState|GetPlayerName _asbp_mordhau_player_state) (Math|Float|Round (Variables|/Script/Engine.PlayerState|GetScore _asbp_mordhau_player_state)) (Variables|/Script/Mordhau.MordhauPlayerState|GetKills _asbp_mordhau_player_state) (Variables|/Script/Mordhau.MordhauPlayerState|GetDeaths _asbp_mordhau_player_state) (Variables|/Script/Mordhau.MordhauPlayerState|GetAssists _asbp_mordhau_player_state)))
      (elif (== (Variables|/Script/Mordhau.MordhauPlayerState|GetTeam _asbp_mordhau_player_state) 1)
        (Utilities|Array|Add (LocalVariables|GetBlue) (Utilities|Struct|MakePlayerInfo (PlayerState|GetPlayerName _asbp_mordhau_player_state) (Math|Float|Round (Variables|/Script/Engine.PlayerState|GetScore _asbp_mordhau_player_state)) (Variables|/Script/Mordhau.MordhauPlayerState|GetKills _asbp_mordhau_player_state) (Variables|/Script/Mordhau.MordhauPlayerState|GetDeaths _asbp_mordhau_player_state) (Variables|/Script/Mordhau.MordhauPlayerState|GetAssists _asbp_mordhau_player_state))))))
  (return (LocalVariables|GetRed) (LocalVariables|GetBlue)))