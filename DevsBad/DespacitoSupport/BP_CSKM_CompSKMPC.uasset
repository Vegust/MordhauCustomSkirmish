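; Player controller for Mordhau's custom skirmish mode, giving players an F7 menu for match settings and admin actions.
; The menu is seeded from the current game state's rules, scores, team names and match log.
; Request events forward settings, score, pause, warmup and round changes to the game state, and match end to the game mode.
; On BeginPlay it loads or creates a client save and adds a persistent HUD widget, which is notified on each character spawn.
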(event Custom|RequestChangeSettings
  (params (Regen :type Boolean) (End :type Integer) (Start :type Integer) (Round :type Integer) (Warmup :type Integer) (MinP :type Integer) (RtW :type Integer) (Late :type Integer) (BlueName :type String) (RedName :type String) (SaveMatch :type Boolean) (IRLDeath :type Boolean) (Scoring :type Boolean))
  (Default|ApplySettings (Variables|Default|GetGameState) Regen End Start Round Warmup MinP RtW Late BlueName RedName SaveMatch IRLDeath Scoring))

(event Custom|RequestSaveStartupSettings
  (Default|SaveStartupSettings (Variables|Default|GetGameState)))

(event Custom|RequestResetScores
  (Default|ServerResetScores (Variables|Default|GetGameState)))

(event Custom|ServerGetScoring
  (bind _asbp_custom_skirmish_game_mode (Utilities|Casting|CastToBP_CustomSkirmishGameMode (Game|GetGameMode)))
  (Variables|Default|Setscoring (Variables|/Script/Mordhau.MordhauGameMode|GetbIsScoringDisabled _asbp_custom_skirmish_game_mode)))

(event Custom|ToggleWidgetPause
  (params (NewPause :type Boolean))
  (Variables|/Game/Mordhau/Maps/CustomSkirmish/UI/SkirmishPersistentWidget.SkirmishPersistentWidget_C|SetPaused (Variables|Default|GetPersistentWidget) NewPause))

(event Custom|ClientInfo
  (Default|InfoLife (Variables|Default|GetPersistentWidget)))

(event Custom|RequestEndMatch
  (bind _asbp_custom_skirmish_game_mode (Utilities|Casting|CastToBP_CustomSkirmishGameMode (Game|GetGameMode)))
  (Class|GameMode|EndMatch _asbp_custom_skirmish_game_mode))

(event Custom|RequestEndRound
  (params (Winner :type Byte))
  (Default|ServerEndRound (Variables|Default|GetGameState) Winner))

(event Custom|RequestChangeScores
  (params (Red :type Integer) (Blue :type Integer))
  (Default|ApplyTeamScores (Variables|Default|GetGameState) Red Blue))

(event Custom|RequestTogglePause
  (params (Paused :type Boolean))
  (Default|ServerTogglePause (Variables|Default|GetGameState) Paused))

(event Custom|RequestSkipWarmup
  (Default|ServerSkipWarmup (Variables|Default|GetGameState)))

(event Custom|LoadClientSave
  (bind _returnvalue (Utilities|String|MakeLiteralString "CustomSkirmish/ClientSave"))
  (bind _returnvalue_2 (SaveGame|DoesSaveGameExist _returnvalue))
  (if _returnvalue_2
    (bind _returnvalue_3 (SaveGame|LoadGamefromSlot _returnvalue))
    (bind _asskirmish_settings_save (Utilities|Casting|CastToSkirmishSettingsSave _returnvalue_3))
    (Variables|Default|SetClientSave _asskirmish_settings_save)
    (else
      (bind _returnvalue_4 (SaveGame|CreateSaveGameObject "/Game/Mordhau/Maps/CustomSkirmish/Saves/SkirmishSettingsSave.SkirmishSettingsSave_C"))
      (Variables|Default|SetClientSave _returnvalue_4)))
  (bind _returnvalue_5 (UserInterface|CreateWidget "/Game/Mordhau/Maps/CustomSkirmish/UI/SkirmishPersistentWidget.SkirmishPersistentWidget_C" self))
  (Variables|Default|SetPersistentWidget _returnvalue_5)
  (UserInterface|Viewport|AddtoViewport _returnvalue_5 0))

(event EventOnMordhauCharacterSpawned
  (params (SpawnedCharacter :type Mordhau%20Character%20Object%20Reference))
  (CallFunction|ClientInfo)
  (|CallParentFunction SpawnedCharacter))

(event EventBeginPlay
  (|CallParentFunction)
  (bind _asbp_custom_skirmish_game_state (Utilities|Casting|CastToBP_CustomSkirmishGameState (Game|GetGameState)))
  (Variables|Default|SetGameState _asbp_custom_skirmish_game_state)
  (CallFunction|LoadClientSave))

(event Input|KeyboardEvents|F7
  (params (Key :type Key%20Structure))
  (:Pressed
    (CallFunction|ShowMenu)))

(fn ConstructionScript
  (|CallParentFunction))

(fn ShowMenu
  (bind _self self)
  (CallFunction|ServerGetScoring)
  (bind _asbp_custom_skirmish_game_state (Utilities|Casting|CastToBP_CustomSkirmishGameState (Game|GetGameState)))
  (bind _returnvalue (UserInterface|CreateWidget "/Game/Mordhau/Maps/CustomSkirmish/UI/CustomSkirmishMainWidget.CustomSkirmishMainWidget_C" _self (Utilities|Array|MakeArray "Contraband" "Contralite" "Terminal" "Bob" "ThePit" "Tourney" "MountainPeak" "Castello" "Feitoria" "Camp" "Grad" "Taiga" "Crossroads" "CompSKM") (Variables|/Script/Mordhau.MordhauGameState|GetbAllowHealthRegen _asbp_custom_skirmish_game_state) (Variables|/Game/Mordhau/Maps/CustomSkirmish/GameModeBlueprints/BP_CustomSkirmishGameState.BP_CustomSkirmishGameState_C|GetEndDur _asbp_custom_skirmish_game_state) (Variables|/Game/Mordhau/Maps/CustomSkirmish/GameModeBlueprints/BP_CustomSkirmishGameState.BP_CustomSkirmishGameState_C|GetStartDur _asbp_custom_skirmish_game_state) (Variables|/Game/Mordhau/Maps/CustomSkirmish/GameModeBlueprints/BP_CustomSkirmishGameState.BP_CustomSkirmishGameState_C|GetRoundDur _asbp_custom_skirmish_game_state) (Variables|/Game/Mordhau/Maps/CustomSkirmish/GameModeBlueprints/BP_CustomSkirmishGameState.BP_CustomSkirmishGameState_C|GetWarmupDur _asbp_custom_skirmish_game_state) (Variables|/Game/Mordhau/Maps/CustomSkirmish/GameModeBlueprints/BP_CustomSkirmishGameState.BP_CustomSkirmishGameState_C|GetMinPl _asbp_custom_skirmish_game_state) (Variables|/Game/Mordhau/Maps/CustomSkirmish/GameModeBlueprints/BP_CustomSkirmishGameState.BP_CustomSkirmishGameState_C|GetRoundsToWin _asbp_custom_skirmish_game_state) (Variables|/Game/Mordhau/Maps/CustomSkirmish/GameModeBlueprints/BP_CustomSkirmishGameState.BP_CustomSkirmishGameState_C|GetLateDur _asbp_custom_skirmish_game_state) (Math|Float|Round (Utilities|Array|Get(acopy) (Variables|/Script/Mordhau.MordhauGameState|GetTeamScores _asbp_custom_skirmish_game_state))) (Math|Float|Round (Utilities|Array|Get(acopy) (Variables|/Script/Mordhau.MordhauGameState|GetTeamScores _asbp_custom_skirmish_game_state) 1)) (Utilities|Array|Get(acopy) (Variables|/Script/Mordhau.MordhauGameState|GetTeamNames _asbp_custom_skirmish_game_state)) (Utilities|Array|Get(acopy) (Variables|/Script/Mordhau.MordhauGameState|GetTeamNames _asbp_custom_skirmish_game_state) 1) (Variables|/Game/Mordhau/Maps/CustomSkirmish/GameModeBlueprints/BP_CustomSkirmishGameState.BP_CustomSkirmishGameState_C|GetSaveMatch _asbp_custom_skirmish_game_state) (Variables|/Game/Mordhau/Maps/CustomSkirmish/GameModeBlueprints/BP_CustomSkirmishGameState.BP_CustomSkirmishGameState_C|GetIRLDeath _asbp_custom_skirmish_game_state) (Variables|/Game/Mordhau/Maps/CustomSkirmish/GameModeBlueprints/BP_CustomSkirmishGameState.BP_CustomSkirmishGameState_C|GetMatchesLog _asbp_custom_skirmish_game_state)))
  (Input|SetInputModeUIOnly _self _returnvalue "DoNotLock")
  (UserInterface|Viewport|AddtoViewport _returnvalue 0)
  (Variables|Default|SetbShowMouseCursor true))