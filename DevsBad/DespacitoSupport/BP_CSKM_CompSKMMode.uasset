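; Custom skirmish game mode for Mordhau (CompSKM) that adds an optional death effect on kills.
; On a kill, if the custom skirmish game state's IRLDeath flag is set, it spawns a BP_Turd at a killed Mordhau character's location before running parent kill handling.
; ReadyToEndMatch simply returns the EndMatch variable, so match end is controlled by that flag.
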(event EventOnKilled
  (params (Killer :type Controller%20Object%20Reference) (KilledPlayer :type Controller%20Object%20Reference) (KilledPawn :type Pawn%20Object%20Reference) (Type :type EMordhauDamageType%20Enum :default "Generic") (SubType :type Byte :default 0) (DamageSource :type Actor%20Object%20Reference) (DamageAgent :type Actor%20Object%20Reference))
  (bind _asbp_custom_skirmish_game_state (Utilities|Casting|CastToBP_CustomSkirmishGameState (Game|GetGameState)))
  (if (Variables|/Game/Mordhau/Maps/CustomSkirmish/GameModeBlueprints/BP_CustomSkirmishGameState.BP_CustomSkirmishGameState_C|GetIRLDeath _asbp_custom_skirmish_game_state)
    (Utilities|Casting|CastToBP_MordhauCharacter KilledPawn
      (:then
        (Game|SpawnActorfromClass "/Game/Mordhau/Blueprints/Equipment/Thrown/BP_Turd.BP_Turd_C" (Math|Conversions|ToTransform(Vector) (Transformation|GetActorLocation KilledPawn)) "AdjustIfPossibleButAlwaysSpawn" 0 0))
      (:CastFailed
        _)))
  (|CallParentFunction Killer KilledPlayer KilledPawn Type SubType DamageSource DamageAgent))

(fn ConstructionScript
  (|CallParentFunction))

(fn ReadytoEndMatch
  (return (Variables|Default|GetEndMatch)))