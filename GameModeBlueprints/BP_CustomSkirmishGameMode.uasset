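; Game mode for a custom Mordhau Skirmish mode that adds kill logging and manual control over match flow.
; Unless scoring is disabled, kills are logged on the killer's player state with victim, round time, location and weapon; the IRLDeath option also spawns a turd at dead characters.
; Game state WarmupPause blocks round starts, and the EndMatch variable alone decides match end.
; Joining players trigger startup and client-info calls on their custom controller.
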(event EventOnKilled
  (params (Killer :type Controller%20Object%20Reference) (KilledPlayer :type Controller%20Object%20Reference) (KilledPawn :type Pawn%20Object%20Reference) (Type :type EMordhauDamageType%20Enum :default "Generic") (SubType :type Byte :default 0) (DamageSource :type Actor%20Object%20Reference) (DamageAgent :type Actor%20Object%20Reference))
  (bind _returnvalue (Transformation|GetActorLocation KilledPawn))
  (bind _playerstate (Variables|/Script/Engine.Controller|GetPlayerState KilledPlayer))
  (bind _playername (Variables|/Script/Engine.PlayerState|GetPlayerName _playerstate))
  (bind _asbp_custom_skirmish_game_state (Utilities|Casting|CastToBP_CustomSkirmishGameState (Game|GetGameState)))
  (Utilities|FlowControl|Sequence
    (:then_0
      (if (not (Variables|Default|GetbIsScoringDisabled))
        (bind _asbp_custom_skirmish_player_state (Utilities|Casting|CastToBP_CustomSkirmishPlayerState (Variables|/Script/Engine.Controller|GetPlayerState Killer)))
        (bind _asmordhau_equipment (Utilities|Casting|CastToMordhauEquipment DamageAgent)
          (:then
            (Default|AddKillevent _asbp_custom_skirmish_player_state _playername (- (GameState|GetServerWorldTimeSeconds _asbp_custom_skirmish_game_state) (.starttime (Variables|/Game/Mordhau/Blueprints/GameModes/Skirmish/BP_SkirmishGameState.BP_SkirmishGameState_C|GetRoundInfo _asbp_custom_skirmish_game_state))) _returnvalue (Utilities|String|ToString(Text) (Variables|/Script/Mordhau.MordhauEquipment|GetEquipmentName _asmordhau_equipment))))
          (:CastFailed
            (Default|AddKillevent _asbp_custom_skirmish_player_state _playername (- (GameState|GetServerWorldTimeSeconds _asbp_custom_skirmish_game_state) (.starttime (Variables|/Game/Mordhau/Blueprints/GameModes/Skirmish/BP_SkirmishGameState.BP_SkirmishGameState_C|GetRoundInfo _asbp_custom_skirmish_game_state))) _returnvalue "None")))))
    (:then_1
      (if (Variables|/Game/Mordhau/Maps/CustomSkirmish/GameModeBlueprints/BP_CustomSkirmishGameState.BP_CustomSkirmishGameState_C|GetIRLDeath _asbp_custom_skirmish_game_state)
        (Utilities|Casting|CastToBP_MordhauCharacter KilledPawn
          (:then
            (Game|SpawnActorfromClass "/Game/Mordhau/Blueprints/Equipment/Thrown/BP_Turd.BP_Turd_C" (Math|Conversions|ToTransform(Vector) (Transformation|GetActorLocation KilledPawn)) "AdjustIfPossibleButAlwaysSpawn" 0 0))
          (:CastFailed
            _)))
      (|CallParentFunction Killer KilledPlayer KilledPawn Type SubType DamageSource DamageAgent))))

(event EventPostLogin
  (params (NewPlayer :type Player%20Controller%20Object%20Reference))
  (bind _asbp_custom_skirmish_player_controller (Utilities|Casting|CastToBP_CustomSkirmishPlayerController NewPlayer))
  (Default|MulticastStart _asbp_custom_skirmish_player_controller)
  (Default|ClientInfo _asbp_custom_skirmish_player_controller))

(event EventBeginPlay
  (|CallParentFunction)
  (bind _asbp_custom_skirmish_game_state (Utilities|Casting|CastToBP_CustomSkirmishGameState (Game|GetGameState)))
  (Variables|Default|SetGameStateC _asbp_custom_skirmish_game_state))

(fn ConstructionScript
  (|CallParentFunction))

(fn ReadytoEndMatch
  (return (Variables|Default|GetEndMatch)))

(fn CanStartRound
  (if (Variables|/Game/Mordhau/Maps/CustomSkirmish/GameModeBlueprints/BP_CustomSkirmishGameState.BP_CustomSkirmishGameState_C|GetWarmupPause (Variables|Default|GetGameStateC))
    (return false)
    (else
      (bind _return (|CallParentFunction))
      (return _return))))