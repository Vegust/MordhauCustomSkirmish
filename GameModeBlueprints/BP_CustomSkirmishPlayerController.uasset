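; Player controller for a Mordhau custom Skirmish mode, providing a match management menu on F7 and a warmup HUD toggle on F8.
; The menu is filled from game state; request events forward settings, score, pause, round and loadout restriction changes there, often logged.
; It also edits or kills players, records damage stats for both sides and suppresses AFK kicks during pauses.
; Kick, ban, unban and slomo requests are empty stubs.
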(event Custom|RequestChangeSettings
  (params (Regen :type Boolean) (End :type Integer) (Start :type Integer) (Round :type Integer) (Warmup :type Integer) (MinP :type Integer) (RtW :type Integer) (Late :type Integer) (BlueName :type String) (RedName :type String) (SaveMatch :type Boolean) (IRLDeath :type Boolean) (Scoring :type Boolean) (Disable%20throwing :type Boolean) (CombatFix :type Boolean))
  (bind _self self)
  (bind _gamestatec (Variables|Default|GetGameStateC))
  (Default|ApplySettings _gamestatec Regen End Start Round Warmup MinP RtW Late BlueName RedName SaveMatch IRLDeath Scoring _self Disable%20throwing CombatFix)
  (Default|MakeLog _gamestatec _self "Applied new skirmish settings."))

(event Custom|RequestSaveStartupSettings
  (Default|SaveStartupSettings (Variables|Default|GetGameStateC) self))

(event Custom|RequestResetScores
  (Default|ServerResetScores (Variables|Default|GetGameStateC) self))

(event Custom|ServerGetScoring
  (bind _asbp_custom_skirmish_game_mode (Utilities|Casting|CastToBP_CustomSkirmishGameMode (Game|GetGameMode)))
  (Variables|Default|Setscoring (Variables|/Script/Mordhau.MordhauGameMode|GetbIsScoringDisabled _asbp_custom_skirmish_game_mode)))

(event Custom|RequestSlomo
  (params (Value :type Float%20%28single-precision%29))
  ;[1 1 1] Crushes the game so i disabled this
)

(event Custom|MulticastStart
  (bind _asbp_custom_skirmish_game_state (Utilities|Casting|CastToBP_CustomSkirmishGameState (Game|GetGameState)))
  (Variables|Default|SetGameStateC _asbp_custom_skirmish_game_state)
  (CallFunction|LoadClientSave))

(event Custom|RequestKick
  (params (SteamID :type Byte) (KickReason :type String))
  ;[1 1 1] Crushes the game so i disabled this
)

(event Custom|RequestBan
  (params (SteamID :type Byte) (BanDuration :type Integer) (BanReason :type String))
  ;[1 1 1] Crushes the game so i disabled this
)

(event Custom|RequestUnban
  (params (SteamID :type Byte))
  ;[1 1 1] Crushes the game so i disabled this
)

(event Custom|RequestPlayerStateChage
  (params (ChangeType :type Integer) (Score :type Integer) (Kills :type Integer) (Deaths :type Integer) (Assists :type Integer) (BanDuration :type Integer) (Target :type BP%20Mordhau%20Player%20State%20Object%20Reference))
  (bind _self self)
  (bind _playername (Variables|/Script/Engine.PlayerState|GetPlayerName Target))
  (switch int ChangeType
    (:0
      (Class|MordhauPlayerState|AddScore Target Score)
      (Class|MordhauPlayerState|AddDeaths Target Deaths)
      (Class|MordhauPlayerState|AddKills Target Kills)
      (Class|MordhauPlayerState|AddAssists Target Assists)
      (Default|MakeLog (Variables|Default|GetGameStateC) self (Utilities|String|JoinStringArray (Utilities|Array|MakeArray "Changed " _playername " stats") " ")))
    (:1
      (Class|AdvancedCharacter|MordhauTakeDamage (Variables|/Script/Mordhau.MordhauPlayerState|GetLastMordhauCharacter Target) 9.99e+03 (Collision|MakeHitResult false false 0.0 0.0 "0, 0, 0" "0, 0, 0" "0,0,1" "0,0,1" 0 0 0 "None" 0 0 "0, 0, 0" "0, 0, 0") "Generic" 0 _self _self)
      (Default|MakeLog (Variables|Default|GetGameStateC) self (Utilities|String|JoinStringArray (Utilities|Array|MakeArray "Killed " _playername) " ")))))

(event Custom|RequestplayerStateSwitchTeam
  (params (New%20team :type Integer) (Target :type BP%20Mordhau%20Player%20State%20Object%20Reference))
  (bind _self self)
  (Variables|/Script/Mordhau.MordhauPlayerState|SetTeam Target New%20team)
  (Default|MakeLog (Variables|Default|GetGameStateC) self (Utilities|String|JoinStringArray (Utilities|Array|MakeArray "Changed " (Variables|/Script/Engine.PlayerState|GetPlayerName Target) " team to " (Utilities|Select :Index (+ New%20team 1) :Option%200 "spectators" :Option%201 "red" :Option%202 "blue")) " "))
  (Class|AdvancedCharacter|MordhauTakeDamage (Variables|/Script/Mordhau.MordhauPlayerState|GetLastMordhauCharacter Target) 9.99e+03 (Collision|MakeHitResult false false 0.0 0.0 "0, 0, 0" "0, 0, 0" "0,0,1" "0,0,1" 0 0 0 "None" 0 0 "0, 0, 0" "0, 0, 0") "Generic" 0 _self _self))

(event Custom|RPCDamageEvent
  (params (type :type EMordhauDamageType%20Enum :default "Generic") (sub%20type :type Byte) (Name :type Name) (Source :type Actor%20Object%20Reference) (Agent :type Actor%20Object%20Reference) (damage :type Float%20%28single-precision%29))
  (Utilities|FlowControl|Sequence
    (:then_0
      (bind _asbp_custom_skirmish_player_state (Utilities|Casting|CastToBP_CustomSkirmishPlayerState (Variables|Default|GetPlayerState)))
      (Default|StatDmgRec _asbp_custom_skirmish_player_state type sub%20type Name Source Agent true damage))
    (:then_1
      (bind _asbp_custom_skirmish_character (Utilities|Casting|CastToBP_CustomSkirmishCharacter Source))
      (bind _asbp_custom_skirmish_player_state_2 (Utilities|Casting|CastToBP_CustomSkirmishPlayerState (Variables|/Script/Engine.Pawn|GetPlayerState _asbp_custom_skirmish_character)))
      (Default|StatDmgRec _asbp_custom_skirmish_player_state_2 type sub%20type Name (Pawn|GetControlledPawn) Agent false damage))))

(event Custom|ToggleWidgetPause
  (params (NewPause :type Boolean))
  (Variables|/Game/Mordhau/Maps/CustomSkirmish/UI/SkirmishPersistentWidget.SkirmishPersistentWidget_C|SetPaused (Variables|Default|GetPersistentWidget) NewPause))

(event Custom|RPCDamageSug
  (params (NewParam :type EMordhauDamageType%20Enum :default "Generic") (NewParam2 :type Byte) (NewParam3 :type Name) (NewParam4 :type Actor%20Object%20Reference) (NewParam5 :type Actor%20Object%20Reference) (NewParam6 :type Float%20%28single-precision%29))
  (CallFunction|RPCDamageEvent NewParam NewParam2 NewParam3 NewParam4 NewParam5 NewParam6))

(event Custom|RequestEquipRestr
  ;[1 1 1] Not used
  (CallFunction|RPCServerBeginWepRestr))

(event Custom|RPCServerBeginWepRestr
  ;[1 1 1] Not used
  (bind _asbp_custom_skirmish_character (Utilities|Casting|CastToBP_CustomSkirmishCharacter (Pawn|GetControlledPawn)))
  (Default|ServerRestrictModes _asbp_custom_skirmish_character))

(event Custom|ApplyLoadoutRestrChanges
  (params (Weapons :type Array%20of%20Mordhau%20Equipment%20Class%20References) (Perks :type Array%20of%20Perk%20Class%20References) (DataList :type Array%20of%20Equipment%20Data%20Object%20References))
  (Default|NewBanArray (Variables|Default|GetGameStateC) Weapons Perks self DataList))

(event Custom|SaveLoadoutRestrChanges
  (Default|SaveStartupBanArray (Variables|Default|GetGameStateC) self))

(event Custom|RequsetWarmupPause
  (bind _gamestatec (Variables|Default|GetGameStateC))
  (Default|ServerBeginWarmup _gamestatec)
  (Default|MakeLog _gamestatec self "Started midgame warmup."))

(event Custom|ClientInfo
  (bind _returnvalue (UserInterface|CreateWidget "/Game/Mordhau/Maps/CustomSkirmish/UI/SkirmishPersistentWidget.SkirmishPersistentWidget_C" self))
  (Variables|Default|SetPersistentWidget _returnvalue)
  (UserInterface|Viewport|AddtoViewport _returnvalue 0)
  (Utilities|FlowControl|Delay 0.2)
  (Default|InfoLife (Variables|Default|GetPersistentWidget)))

(event Custom|RequestEndMatch
  (bind _asbp_custom_skirmish_game_mode (Utilities|Casting|CastToBP_CustomSkirmishGameMode (Game|GetGameMode)))
  (Class|GameMode|EndMatch _asbp_custom_skirmish_game_mode))

(event Custom|RequestEndRound
  (params (Winner :type Byte))
  (Default|ServerEndRound (Variables|Default|GetGameStateC) Winner self))

(event Custom|RequestChangeScores
  (params (Red :type Integer) (Blue :type Integer))
  (Default|ApplyTeamScores (Variables|Default|GetGameStateC) Red Blue self))

(event Custom|RequestTogglePause
  (params (Paused :type Boolean))
  (bind _self self)
  (bind _gamestatec (Variables|Default|GetGameStateC))
  (Utilities|FlowControl|Sequence
    (:then_0
      (if Paused
        (Class|MordhauPlayerController|ServerSlomo 0.0)
        (else
          (Class|MordhauPlayerController|ServerSlomo 1.0)))
      (Default|ServerTogglePause _gamestatec Paused _self))
    (:then_1
      (Default|MakeLog _gamestatec _self (select Paused "Paused the game." "Unpaused the game.")))))

(event Custom|RequestSkipWarmup
  (bind _self self)
  (bind _gamestatec (Variables|Default|GetGameStateC))
  (Default|ServerSkipWarmup _gamestatec _self)
  (Default|MakeLog _gamestatec _self "Skipped match to round start."))

(event Custom|LoadClientSave
  (bind _returnvalue (Utilities|String|MakeLiteralString "CustomSkirmish/ClientSave"))
  (bind _returnvalue_2 (SaveGame|DoesSaveGameExist _returnvalue))
  (if _returnvalue_2
    (bind _returnvalue_3 (SaveGame|LoadGamefromSlot _returnvalue))
    (bind _asskirmish_settings_save (Utilities|Casting|CastToSkirmishSettingsSave _returnvalue_3))
    (Variables|Default|SetClientSaveC _asskirmish_settings_save)
    (else
      (bind _returnvalue_4 (SaveGame|CreateSaveGameObject "/Game/Mordhau/Maps/CustomSkirmish/Saves/SkirmishSettingsSave.SkirmishSettingsSave_C"))
      (Variables|Default|SetClientSaveC _returnvalue_4))))

(event EventOnAFKTimeExceededMaximum
  (bind _gamestatec (Variables|Default|GetGameStateC))
  (if (Variables|/Game/Mordhau/Maps/CustomSkirmish/GameModeBlueprints/BP_CustomSkirmishGameState.BP_CustomSkirmishGameState_C|GetGamePaused _gamestatec)
    (Variables|Default|SetCurrentAFKTime 0.0 :!label _label)
    (elif (Variables|/Game/Mordhau/Maps/CustomSkirmish/GameModeBlueprints/BP_CustomSkirmishGameState.BP_CustomSkirmishGameState_C|GetWarmupPause _gamestatec)
      (goto _label)
      (else
        (CallFunction|PerformAFKKick)))))

(event EventPerformAFKKick
  (bind _gamestatec (Variables|Default|GetGameStateC))
  (if (not (or (Variables|/Game/Mordhau/Maps/CustomSkirmish/GameModeBlueprints/BP_CustomSkirmishGameState.BP_CustomSkirmishGameState_C|GetGamePaused _gamestatec) (Variables|/Game/Mordhau/Maps/CustomSkirmish/GameModeBlueprints/BP_CustomSkirmishGameState.BP_CustomSkirmishGameState_C|GetWarmupPause _gamestatec)))
    (|CallParentFunction)))

(event Input|KeyboardEvents|F7
  (params (Key :type Key%20Structure))
  (:Pressed
    (CallFunction|ShowMenu)))

(event Input|KeyboardEvents|F8
  (params (Key :type Key%20Structure))
  (:Pressed
    (if (Variables|Default|GetHideWarmupHud)
      (Variables|Default|SetHideWarmupHud false)
      (else
        (Variables|Default|SetHideWarmupHud true)))))

(fn ConstructionScript
  (|CallParentFunction))

(fn ShowMenu
  (bind _self self)
  (CallFunction|ServerGetScoring)
  (bind _asbp_custom_skirmish_game_state (Utilities|Casting|CastToBP_CustomSkirmishGameState (Game|GetGameState)))
  (bind _returnvalue (UserInterface|CreateWidget "/Game/Mordhau/Maps/CustomSkirmish/UI/CustomSkirmishMainWidget.CustomSkirmishMainWidget_C" _self (Utilities|Array|MakeArray "Contraband" "Contralite" "Terminal" "Bob" "ThePit" "Tourney" "MountainPeak" "Castello" "Feitoria" "Camp" "Grad" "Taiga" "Crossroads" "CompSKM (test version)" "Contrabob" "RockStand" "Chester" "Steedie_Contraband" "RackStand" "Moshpit") (Variables|/Game/Mordhau/Maps/CustomSkirmish/GameModeBlueprints/BP_CustomSkirmishGameState.BP_CustomSkirmishGameState_C|GetRegenSetting _asbp_custom_skirmish_game_state) (Variables|/Game/Mordhau/Maps/CustomSkirmish/GameModeBlueprints/BP_CustomSkirmishGameState.BP_CustomSkirmishGameState_C|GetEndDur _asbp_custom_skirmish_game_state) (Variables|/Game/Mordhau/Maps/CustomSkirmish/GameModeBlueprints/BP_CustomSkirmishGameState.BP_CustomSkirmishGameState_C|GetStartDur _asbp_custom_skirmish_game_state) (Variables|/Game/Mordhau/Maps/CustomSkirmish/GameModeBlueprints/BP_CustomSkirmishGameState.BP_CustomSkirmishGameState_C|GetRoundDur _asbp_custom_skirmish_game_state) (Variables|/Game/Mordhau/Maps/CustomSkirmish/GameModeBlueprints/BP_CustomSkirmishGameState.BP_CustomSkirmishGameState_C|GetWarmupDur _asbp_custom_skirmish_game_state) (Variables|/Game/Mordhau/Maps/CustomSkirmish/GameModeBlueprints/BP_CustomSkirmishGameState.BP_CustomSkirmishGameState_C|GetMinPl _asbp_custom_skirmish_game_state) (Variables|/Game/Mordhau/Maps/CustomSkirmish/GameModeBlueprints/BP_CustomSkirmishGameState.BP_CustomSkirmishGameState_C|GetRoundsToWin _asbp_custom_skirmish_game_state) (Variables|/Game/Mordhau/Maps/CustomSkirmish/GameModeBlueprints/BP_CustomSkirmishGameState.BP_CustomSkirmishGameState_C|GetLateDur _asbp_custom_skirmish_game_state) (Math|Float|Round (Utilities|Array|Get(acopy) (Variables|/Script/Mordhau.MordhauGameState|GetTeamScores _asbp_custom_skirmish_game_state))) (Math|Float|Round (Utilities|Array|Get(acopy) (Variables|/Script/Mordhau.MordhauGameState|GetTeamScores _asbp_custom_skirmish_game_state) 1)) (Utilities|Array|Get(acopy) (Variables|/Script/Mordhau.MordhauGameState|GetTeamNames _asbp_custom_skirmish_game_state)) (Utilities|Array|Get(acopy) (Variables|/Script/Mordhau.MordhauGameState|GetTeamNames _asbp_custom_skirmish_game_state) 1) (Variables|/Game/Mordhau/Maps/CustomSkirmish/GameModeBlueprints/BP_CustomSkirmishGameState.BP_CustomSkirmishGameState_C|GetSaveMatch _asbp_custom_skirmish_game_state) (Variables|/Game/Mordhau/Maps/CustomSkirmish/GameModeBlueprints/BP_CustomSkirmishGameState.BP_CustomSkirmishGameState_C|GetIRLDeath _asbp_custom_skirmish_game_state) (Variables|/Game/Mordhau/Maps/CustomSkirmish/GameModeBlueprints/BP_CustomSkirmishGameState.BP_CustomSkirmishGameState_C|GetMatchesLog _asbp_custom_skirmish_game_state) (Variables|/Game/Mordhau/Maps/CustomSkirmish/GameModeBlueprints/BP_CustomSkirmishGameState.BP_CustomSkirmishGameState_C|GetLogArray _asbp_custom_skirmish_game_state) 0 (Variables|/Game/Mordhau/Maps/CustomSkirmish/GameModeBlueprints/BP_CustomSkirmishGameState.BP_CustomSkirmishGameState_C|GetDisable%20throwing _asbp_custom_skirmish_game_state) (Variables|/Game/Mordhau/Maps/CustomSkirmish/GameModeBlueprints/BP_CustomSkirmishGameState.BP_CustomSkirmishGameState_C|GetreplicatedBanPerksArray _asbp_custom_skirmish_game_state) (Variables|/Game/Mordhau/Maps/CustomSkirmish/GameModeBlueprints/BP_CustomSkirmishGameState.BP_CustomSkirmishGameState_C|GetreplicatedBanArray _asbp_custom_skirmish_game_state) (Variables|/Game/Mordhau/Maps/CustomSkirmish/GameModeBlueprints/BP_CustomSkirmishGameState.BP_CustomSkirmishGameState_C|GetEquipmentDataList _asbp_custom_skirmish_game_state) (Variables|/Game/Mordhau/Maps/CustomSkirmish/GameModeBlueprints/BP_CustomSkirmishGameState.BP_CustomSkirmishGameState_C|GetCombatFix _asbp_custom_skirmish_game_state)))
  (Variables|Default|SetMainWidget _returnvalue)
  (Input|SetInputModeUIOnly _self _returnvalue "DoNotLock")
  (UserInterface|Viewport|AddtoViewport _returnvalue 0)
  (Variables|Default|SetbShowMouseCursor true))