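; Skirmish player state that records per-round combat statistics for each player on the server, for Scalagrad servers.
; Tick polls the last character's NetBlock while scoring is enabled, tallies parries, chambers, clashes and feint-to-parries, then clears it to detect new blocks.
; Event entry points accumulate kills and hit/damage totals by body region and type.
; The round-end callback adds armor, perks, equipment and outcome, archives the record, then resets it.
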(event Custom|AddKillevent
  (params (Victim :type String) (Time :type Float%20%28single-precision%29) (Location :type Vector) (Weapon :type String))
  (Utilities|Array|Add (.kilevents (Variables|Default|GetCurrentRoundStats)) (Utilities|Struct|MakeSkirmishKillEvent Victim Time Location Weapon)))

(event Custom|RoundEndChange
  (params (Round :type Integer) (WinnerTeam :type Integer))
  (bind _tmpequipmentarray (Variables|Default|GetTmpEquipmentArray))
  (bind _lastmordhaucharacter (Variables|Default|GetLastMordhauCharacter))
  (bind _mesh (Variables|/Script/Engine.Character|GetMesh _lastmordhaucharacter))
  (if (Variables|/Game/Mordhau/Maps/CustomSkirmish/GameModeBlueprints/BP_CustomSkirmishGameState.BP_CustomSkirmishGameState_C|GetIsScalagradServer (Variables|Default|GetGameState))
    (Utilities|FlowControl|Delay 0.1)
    (bind _returnvalue (Class|AdvancedCharacter|GetArmorTierforBone _lastmordhaucharacter (Class|SkinnedMeshComponent|GetSocketBoneName _mesh "Head")))
    (bind _returnvalue_2 (Class|AdvancedCharacter|GetArmorTierforBone _lastmordhaucharacter (Class|SkinnedMeshComponent|GetSocketBoneName _mesh "Spine")))
    (bind _returnvalue_3 (Class|AdvancedCharacter|GetArmorTierforBone _lastmordhaucharacter (Class|SkinnedMeshComponent|GetSocketBoneName _mesh "LeftLeg")))
    (Utilities|Array|Clear (Variables|Default|GetTmpPerkArray))
    (for _index (range 0 18)
      (bind _returnvalue_4 (Class|MordhauCharacter|HasPerk _lastmordhaucharacter (Math|Conversions|ToByte(Integer) _index)))
      (if _returnvalue_4
        (Utilities|Array|Add (Variables|Default|GetTmpPerkArray) (Utilities|String|ToString(Integer) _index))))
    (Utilities|Array|Clear _tmpequipmentarray)
    (for _array_element (.Equipment (Utilities|Struct|BreakCharacterGearCustomization (.GearCustomization (Utilities|Struct|BreakCharacterProfile (Variables|/Script/Mordhau.MordhauCharacter|GetProfile _lastmordhaucharacter)))))
      (Utilities|Array|Add _tmpequipmentarray (.ID (Utilities|Struct|BreakEquipmentCustomization _array_element))))
    (bind _asbp_custom_skirmish_game_state (Utilities|Casting|CastToBP_CustomSkirmishGameState (Game|GetGameState)))
    (bind _output_get (Variables|Default|SetCurrentRoundStats (Utilities|Struct|MakePlayerRoundStats (.roundnumber (Variables|Default|GetCurrentRoundStats)) (Utilities|Struct|MakeIntVector (Math|Conversions|ToInteger(Byte) _returnvalue) (Math|Conversions|ToInteger(Byte) _returnvalue_2) (Math|Conversions|ToInteger(Byte) _returnvalue_3)) (== (Variables|Default|GetTeam) (Math|Conversions|ToInteger(Byte) (Variables|/Game/Mordhau/Blueprints/GameModes/Skirmish/BP_SkirmishGameState.BP_SkirmishGameState_C|GetLastWinner _asbp_custom_skirmish_game_state))) (Variables|Default|GetbIsAlive) (GameState|GetServerWorldTimeSeconds _asbp_custom_skirmish_game_state) (Variables|Default|GetTmpPerkArray) (Variables|Default|GetTmpEquipmentArray) (.kilevents (Variables|Default|GetCurrentRoundStats)) (.blockinfo (Variables|Default|GetCurrentRoundStats)) (Variables|Default|GetRoundDealt) (Variables|Default|GetRoundRecieved))))
    (Utilities|Array|Add (Variables|Default|GetPlayedRoundsStats) _output_get)
    (Variables|Default|SetCurrentRoundStats (Utilities|Struct|MakePlayerRoundStats Round (Utilities|Struct|MakeIntVector 0 0 0) false false 0.0 (Utilities|Array|MakeArray) (Utilities|Array|MakeArray) (Utilities|Array|MakeArray) (Utilities|Struct|MakeSkirmishRoundBlockInfoStruct 0 0 0 0 0 0 0 0) "(HitsTotal_19_7167A1A3496E6D7F05DAB2866901282B=0,DamageTotal_32_E2AA131242E28DCFE9C5CFA855F7734E=0,HeadHits_33_3B6B26B24A81F44A0A0489AD9019CD31=0,TorsoHits_34_5D2BCC494B1AB178C04CD495514CF8F3=0,LegHits_35_41BBC18049DCBB6D1963A38BD620C674=0,RangedDamage_36_7D51ADA24AF008759E650EBE7C3EEBAF=0,FireDamage_37_ECD9ABE0475C8B6D272305B6EE948891=0)" "(HitsTotal_19_7167A1A3496E6D7F05DAB2866901282B=0,DamageTotal_32_E2AA131242E28DCFE9C5CFA855F7734E=0,HeadHits_33_3B6B26B24A81F44A0A0489AD9019CD31=0,TorsoHits_34_5D2BCC494B1AB178C04CD495514CF8F3=0,LegHits_35_41BBC18049DCBB6D1963A38BD620C674=0,RangedDamage_36_7D51ADA24AF008759E650EBE7C3EEBAF=0,FireDamage_37_ECD9ABE0475C8B6D272305B6EE948891=0)"))
    (Variables|Default|SetRoundDealt (Utilities|Struct|MakeSkirmishRoundDamageInfoStruct 0 0 0 0 0 0 0))
    (Variables|Default|SetRoundRecieved (Utilities|Struct|MakeSkirmishRoundDamageInfoStruct 0 0 0 0 0 0 0))))

(event Custom|StatDmgRec
  (params (Type :type EMordhauDamageType%20Enum :default "Generic") (SubType :type Byte) (Bone :type Name) (Source :type Actor%20Object%20Reference) (Agent :type Actor%20Object%20Reference) (Recieved :type Boolean) (Damage :type Float%20%28single-precision%29))
  (bind _returnvalue (Math|Float|Round Damage))
  (bind _returnvalue_2 (Utilities|Select :Index Type :Generic 1 :Melee 1 :Ranged 1 :Fall 1 :Fire 0))
  (bind _returnvalue_3 (Class|KismetSystemLibrary|MakeLiteralInteger _returnvalue_2))
  (bind _returnvalue_4 (Utilities|Select :Index Type :Generic 0 :Melee 0 :Ranged 0 :Fall 0 :Fire _returnvalue))
  (bind _returnvalue_5 (Utilities|Select :Index Type :Generic 0 :Melee _returnvalue :Ranged _returnvalue :Fall _returnvalue :Fire _returnvalue))
  (bind _returnvalue_6 (Utilities|Select :Index Type :Generic 0 :Melee 0 :Ranged _returnvalue :Fall 0 :Fire 0))
  (if (not (Variables|/Script/Mordhau.MordhauGameMode|GetbIsScoringDisabled (Variables|Default|GetGameMode)))
    (bind _returnvalue_7 (Class|MordhauCharacter|IsHead Bone))
    (bind _returnvalue_8 (Class|MordhauCharacter|IsLeg Bone))
    (bind _returnvalue_9 (Class|MordhauCharacter|IsArm Bone))
    (if (not Recieved)
      (Variables|Default|SetRoundRecieved (Utilities|Struct|MakeSkirmishRoundDamageInfoStruct (+ (.hitstotal (Variables|Default|GetRoundRecieved)) _returnvalue_3) (+ (.damagetotal (Variables|Default|GetRoundRecieved)) _returnvalue_5) (+ (.headhits (Variables|Default|GetRoundRecieved)) (Math|Integer|SelectInt _returnvalue_2 0 _returnvalue_7)) (+ (.torsohits (Variables|Default|GetRoundRecieved)) (Math|Integer|SelectInt _returnvalue_2 0 (or _returnvalue_9 (not (or _returnvalue_7 _returnvalue_8))))) (+ (.leghits (Variables|Default|GetRoundRecieved)) (Math|Integer|SelectInt _returnvalue_2 0 _returnvalue_8)) (+ (.rangeddamage (Variables|Default|GetRoundRecieved)) _returnvalue_6) (+ (.firedamage (Variables|Default|GetRoundRecieved)) _returnvalue_4)))
      (else
        (Variables|Default|SetRoundDealt (Utilities|Struct|MakeSkirmishRoundDamageInfoStruct (+ (.hitstotal (Variables|Default|GetRoundDealt)) _returnvalue_3) (+ (.damagetotal (Variables|Default|GetRoundDealt)) _returnvalue_5) (+ (.headhits (Variables|Default|GetRoundDealt)) (Math|Integer|SelectInt _returnvalue_2 0 _returnvalue_7)) (+ (.torsohits (Variables|Default|GetRoundDealt)) (Math|Integer|SelectInt _returnvalue_2 0 (or _returnvalue_9 (not (or _returnvalue_7 _returnvalue_8))))) (+ (.leghits (Variables|Default|GetRoundDealt)) (Math|Integer|SelectInt _returnvalue_2 0 _returnvalue_8)) (+ (.rangeddamage (Variables|Default|GetRoundDealt)) _returnvalue_6) (+ (.firedamage (Variables|Default|GetRoundDealt)) _returnvalue_4)))))))

(event EventBeginPlay
  (Networking|SwitchHasAuthority
    (:Authority
      (bind _asbp_custom_skirmish_game_state (Utilities|Casting|CastToBP_CustomSkirmishGameState (Game|GetGameState)))
      (Variables|Default|SetGameState _asbp_custom_skirmish_game_state)
      (EventDispatchers|BindEventtoRoundEndEvent _asbp_custom_skirmish_game_state (delegate Custom|RoundEndChange))
      (bind _asbp_custom_skirmish_game_mode (Utilities|Casting|CastToBP_CustomSkirmishGameMode (Game|GetGameMode)))
      (Variables|Default|SetGameMode _asbp_custom_skirmish_game_mode))))

(event EventTick
  (params (DeltaSeconds :type Float%20%28single-precision%29))
  (bind _lastmordhaucharacter (Variables|Default|GetLastMordhauCharacter))
  (bind _lastfeintedmotion (Variables|/Script/Mordhau.MordhauCharacter|GetLastFeintedMotion _lastmordhaucharacter))
  (bind _lastparrymotion (Variables|/Script/Mordhau.MordhauCharacter|GetLastParryMotion _lastmordhaucharacter))
  (bind _starttime (Variables|/Script/Mordhau.MordhauMotion|GetStartTime _lastfeintedmotion))
  (bind _starttime_2 (Variables|/Script/Mordhau.MordhauMotion|GetStartTime _lastparrymotion))
  (|CallParentFunction DeltaSeconds)
  (Networking|SwitchHasAuthority
    (:Authority
      (if (Variables|/Game/Mordhau/Maps/CustomSkirmish/GameModeBlueprints/BP_CustomSkirmishGameState.BP_CustomSkirmishGameState_C|GetIsScalagradServer (Variables|Default|GetGameState))
        (if (not (Variables|/Script/Mordhau.MordhauGameMode|GetbIsScoringDisabled (Variables|Default|GetGameMode)))
          (if (Math|Boolean|ANDBoolean (== 0 (.blockedreason (Variables|/Script/Mordhau.MordhauCharacter|GetNetBlock _lastmordhaucharacter))) (== 0 (.blockedmove (Variables|/Script/Mordhau.MordhauCharacter|GetNetBlock _lastmordhaucharacter))) (== 0 (.blocktype (Variables|/Script/Mordhau.MordhauCharacter|GetNetBlock _lastmordhaucharacter))) (== 0 (.blockedangle (Variables|/Script/Mordhau.MordhauCharacter|GetNetBlock _lastmordhaucharacter))))
            (Variables|Default|SetLastEasyParryTime (Variables|/Script/Mordhau.MordhauCharacter|GetEasyParryUntilTime _lastmordhaucharacter))
            (else
              (Variables|Default|SetCurrentRoundStats (Utilities|Struct|MakePlayerRoundStats (.roundnumber (Variables|Default|GetCurrentRoundStats)) (.armorvalues (Variables|Default|GetCurrentRoundStats)) (.wonround (Variables|Default|GetCurrentRoundStats)) (.aliveattheend (Variables|Default|GetCurrentRoundStats)) (.roundduration (Variables|Default|GetCurrentRoundStats)) (.perkslist (Variables|Default|GetCurrentRoundStats)) (.equipmentlist (Variables|Default|GetCurrentRoundStats)) (.kilevents (Variables|Default|GetCurrentRoundStats)) (Utilities|Struct|MakeSkirmishRoundBlockInfoStruct (select (Utilities|Select :Index (Math|Conversions|ToInteger(Byte) (.BlockedReason (Utilities|Struct|BreakNetBlock (Variables|/Script/Mordhau.MordhauCharacter|GetNetBlock _lastmordhaucharacter)))) :Option%200 true :Option%201 true :Option%202 true :Option%203 false :Option%204 false :Option%205 false :Option%206 false :Option%207 false :Option%208 false :Option%209 false :Option%2010 false :Option%2011 false :Option%2012 true :Option%2013 false :Option%2014 false) (+ (.parriestotal (.blockinfo (Variables|Default|GetCurrentRoundStats))) 1) (.parriestotal (.blockinfo (Variables|Default|GetCurrentRoundStats)))) (select (Utilities|Select :Index (Math|Conversions|ToInteger(Byte) (.BlockedReason (Utilities|Struct|BreakNetBlock (Variables|/Script/Mordhau.MordhauCharacter|GetNetBlock _lastmordhaucharacter)))) :Option%200 false :Option%201 false :Option%202 false :Option%203 true :Option%204 true :Option%205 false :Option%206 false :Option%207 false :Option%208 false :Option%209 false :Option%2010 false :Option%2011 false :Option%2012 false :Option%2013 false :Option%2014 false) (+ (.chaberstotal (.blockinfo (Variables|Default|GetCurrentRoundStats))) 1) (.chaberstotal (.blockinfo (Variables|Default|GetCurrentRoundStats)))) (select (and (or (Utilities|Select :Index (Math|Conversions|ToInteger(Byte) (.BlockedReason (Utilities|Struct|BreakNetBlock (Variables|/Script/Mordhau.MordhauCharacter|GetNetBlock _lastmordhaucharacter)))) :Option%200 false :Option%201 false :Option%202 false :Option%203 true :Option%204 true :Option%205 false :Option%206 false :Option%207 false :Option%208 false :Option%209 false :Option%2010 false :Option%2011 false :Option%2012 false :Option%2013 false :Option%2014 false) (Utilities|Select :Index (Math|Conversions|ToInteger(Byte) (.BlockedReason (Utilities|Struct|BreakNetBlock (Variables|/Script/Mordhau.MordhauCharacter|GetNetBlock _lastmordhaucharacter)))) :Option%200 true :Option%201 true :Option%202 true :Option%203 false :Option%204 false :Option%205 false :Option%206 false :Option%207 false :Option%208 false :Option%209 false :Option%2010 false :Option%2011 false :Option%2012 true :Option%2013 false :Option%2014 false)) (> (- (Variables|Default|GetLastEasyParryTime) (GameState|GetServerWorldTimeSeconds (Game|GetGameState))) 0.0)) (+ (.parriesduringeasyparrywindow (.blockinfo (Variables|Default|GetCurrentRoundStats))) 1) (.parriesduringeasyparrywindow (.blockinfo (Variables|Default|GetCurrentRoundStats)))) (select (Utilities|Select :Index (Math|Conversions|ToInteger(Byte) (.BlockedReason (Utilities|Struct|BreakNetBlock (Variables|/Script/Mordhau.MordhauCharacter|GetNetBlock _lastmordhaucharacter)))) :Option%200 false :Option%201 false :Option%202 false :Option%203 false :Option%204 false :Option%205 false :Option%206 true :Option%207 true :Option%208 false :Option%209 false :Option%2010 false :Option%2011 false :Option%2012 false :Option%2013 false :Option%2014 true) (+ (.clashes (.blockinfo (Variables|Default|GetCurrentRoundStats))) 1) (.clashes (.blockinfo (Variables|Default|GetCurrentRoundStats)))) (select (Utilities|Select :Index (Math|Conversions|ToInteger(Byte) (.BlockedReason (Utilities|Struct|BreakNetBlock (Variables|/Script/Mordhau.MordhauCharacter|GetNetBlock _lastmordhaucharacter)))) :Option%200 false :Option%201 true :Option%202 false :Option%203 false :Option%204 false :Option%205 false :Option%206 false :Option%207 false :Option%208 false :Option%209 false :Option%2010 false :Option%2011 false :Option%2012 false :Option%2013 false :Option%2014 false) (+ (.disarmingparries (.blockinfo (Variables|Default|GetCurrentRoundStats))) 1) (.disarmingparries (.blockinfo (Variables|Default|GetCurrentRoundStats)))) (select (Utilities|Select :Index (Math|Conversions|ToInteger(Byte) (.BlockedMove (Utilities|Struct|BreakNetBlock (Variables|/Script/Mordhau.MordhauCharacter|GetNetBlock _lastmordhaucharacter)))) :Option%200 false :Option%201 false :Option%202 false :Option%203 false :Option%204 true :Option%205 false :Option%206 false :Option%207 false) (+ (.blockedkicks (.blockinfo (Variables|Default|GetCurrentRoundStats))) 1) (.blockedkicks (.blockinfo (Variables|Default|GetCurrentRoundStats)))) (select (Utilities|Select :Index (Math|Conversions|ToInteger(Byte) (.BlockedMove (Utilities|Struct|BreakNetBlock (Variables|/Script/Mordhau.MordhauCharacter|GetNetBlock _lastmordhaucharacter)))) :Option%200 false :Option%201 false :Option%202 false :Option%203 false :Option%204 false :Option%205 false :Option%206 false :Option%207 true) (+ (.blockedprojectiles (.blockinfo (Variables|Default|GetCurrentRoundStats))) 1) (.blockedprojectiles (.blockinfo (Variables|Default|GetCurrentRoundStats)))) (select (and (Math|Boolean|ANDBoolean (< (Math|Float|Absolute(Float) (- _starttime _starttime_2)) 0.4) (!= _starttime_2 0.0) (!= 0.0 _starttime)) (Utilities|Select :Index (Math|Conversions|ToInteger(Byte) (.BlockedReason (Utilities|Struct|BreakNetBlock (Variables|/Script/Mordhau.MordhauCharacter|GetNetBlock _lastmordhaucharacter)))) :Option%200 true :Option%201 true :Option%202 true :Option%203 false :Option%204 false :Option%205 false :Option%206 false :Option%207 false :Option%208 false :Option%209 false :Option%2010 false :Option%2011 false :Option%2012 true :Option%2013 false :Option%2014 false)) (+ (.feintstoparry (.blockinfo (Variables|Default|GetCurrentRoundStats))) 1) (.feintstoparry (.blockinfo (Variables|Default|GetCurrentRoundStats))))) (.damagedealtinfo (Variables|Default|GetCurrentRoundStats)) (.damagerecievedinfo (Variables|Default|GetCurrentRoundStats))))
              (Variables|/Script/Mordhau.MordhauCharacter|SetNetBlock _lastmordhaucharacter (Utilities|Struct|MakeNetBlock 0 0 0 0 0 0)))))))))

(fn ConstructionScript
  (|CallParentFunction))