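; Player character for Mordhau custom Skirmish that enforces game state restrictions and reports damage stats.
; While DisableThrowing is set, Tick clears AllowFire on weapons and shields, and once, after a short delay, strips perks from profiles holding banned ones.
; Authority caches damage taken; on Scalagrad servers, hits go to the custom player controller by RPC, or without one are recorded directly on victim and attacker player states.
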(event Custom|ServerDamageStat
  (params (type :type EMordhauDamageType%20Enum :default "Generic") (sub%20type :type Byte) (bone :type Name) (source :type Actor%20Object%20Reference) (agent :type Actor%20Object%20Reference))
  (bind _lasttakendamage (Variables|Default|GetLastTakenDamage))
  (Utilities|FlowControl|Sequence
    (:then_0
      (bind _asbp_custom_skirmish_player_state (Utilities|Casting|CastToBP_CustomSkirmishPlayerState (Variables|Default|GetPlayerState)))
      (Default|StatDmgRec _asbp_custom_skirmish_player_state type sub%20type bone source agent true _lasttakendamage))
    (:then_1
      (bind _asbp_custom_skirmish_character (Utilities|Casting|CastToBP_CustomSkirmishCharacter source))
      (bind _asbp_custom_skirmish_player_state_2 (Utilities|Casting|CastToBP_CustomSkirmishPlayerState (Variables|/Script/Engine.Pawn|GetPlayerState _asbp_custom_skirmish_character)))
      (Default|StatDmgRec _asbp_custom_skirmish_player_state_2 type sub%20type bone self agent false _lasttakendamage))))

(event Custom|ServerRestrictModes
  ;[1 1 1] this shit does not work so i guess i will add another ticking function :--00-0-0____)))))))))))))))))))))))))
  (CallFunction|DisableThrowing (Variables|Default|GetEquipment)))

(event EventMordhauDamage
  (params (Damage :type Float%20%28single-precision%29) (HitResult :type Hit%20Result%20Structure%20%28by%20ref%29) (DamageType :type EMordhauDamageType%20Enum :default "Generic") (SubDamageType :type Byte :default 0) (Source :type Actor%20Object%20Reference) (Agent :type Actor%20Object%20Reference) (EventInstigator :type Controller%20Object%20Reference))
  (|CallParentFunction Damage HitResult DamageType SubDamageType Source Agent EventInstigator)
  (Networking|SwitchHasAuthority
    (:Authority
      (Variables|Default|SetLastTakenDamage Damage))))

(event EventOnPostProfileAssigned
  ;[1 1 1] this shit does not work so i guess i will add another ticking function :--00-0-0____)))))))))))))))))))))))))
  (|CallParentFunction))

(event EventOnPickedUp
  (params (Eq :type Mordhau%20Equipment%20Object%20Reference))
  ;[1 1 1] this shit does not work so i guess i will add another ticking function :--00-0-0____)))))))))))))))))))))))))
  (|CallParentFunction Eq))

(event EventTick
  (params (DeltaSeconds :type Float%20%28single-precision%29))
  (|CallParentFunction DeltaSeconds)
  (if (Variables|/Game/Mordhau/Maps/CustomSkirmish/GameModeBlueprints/BP_CustomSkirmishGameState.BP_CustomSkirmishGameState_C|GetDisable%20throwing (Variables|Default|GetGameState))
    (CallFunction|DisableThrowing (Variables|Default|GetEquipment))
    (Utilities|FlowControl|DoOnce false
      (:Completed
        (Utilities|FlowControl|Delay 0.2)
        (for _array_element (Variables|/Game/Mordhau/Maps/CustomSkirmish/GameModeBlueprints/BP_CustomSkirmishGameState.BP_CustomSkirmishGameState_C|GetreplicatedBanPerksArray (Variables|Default|GetGameState))
          (bind _returnvalue (Class|MordhauCharacter|HasPerk (Math|Conversions|ToByte(Integer) (Utilities|Array|FindItem (Variables|Default|GetAllPerks) _array_element))))
          (if _returnvalue
            (bind _output_get (Variables|Default|SetProfile (Class|MordhauUtilityLibrary|StripProfile (Variables|Default|GetProfile) false true false)))
            (Class|MordhauCharacter|AssignProfile self _output_get)))))))

(event EventBeginPlay
  (|CallParentFunction)
  (bind _asbp_custom_skirmish_game_state (Utilities|Casting|CastToBP_CustomSkirmishGameState (Game|GetGameState)))
  (Variables|Default|SetGameState _asbp_custom_skirmish_game_state))

(event EventOnTookDamage
  (params (bWillKill :type Boolean) (Type :type EMordhauDamageType%20Enum :default "Generic") (SubType :type Byte :default 0) (bone :type Name%20%28by%20ref%29 :default "None") (Point :type Vector%20%28by%20ref%29 :default "0, 0, 0") (Source :type Actor%20Object%20Reference) (Agent :type Actor%20Object%20Reference))
  (|CallParentFunction bWillKill Type SubType bone Point Source Agent)
  (if (Variables|/Game/Mordhau/Maps/CustomSkirmish/GameModeBlueprints/BP_CustomSkirmishGameState.BP_CustomSkirmishGameState_C|GetIsScalagradServer (Variables|Default|GetGameState))
    (Utilities|FlowControl|Delay 0.0)
    (bind _asbp_custom_skirmish_player_controller (Utilities|Casting|CastToBP_CustomSkirmishPlayerController (Pawn|GetController))
      (:then
        (Default|RPCDamageSug _asbp_custom_skirmish_player_controller Type SubType bone Source Agent (Variables|Default|GetLastTakenDamage)))
      (:CastFailed
        (CallFunction|ServerDamageStat Type SubType bone Source Agent)))))

(fn ConstructionScript
  (|CallParentFunction))

(fn DisableThrowing
  (params (Array :type Array%20of%20Mordhau%20Equipment%20Object%20References))
  (for _array_element Array
    (if (or (Utilities|ClassIsChildOf (Utilities|GetClass _array_element) "/Script/Mordhau.MordhauWeapon") (Utilities|ClassIsChildOf (Utilities|GetClass _array_element) "/Script/Mordhau.MordhauShield"))
      (Variables|/Script/Mordhau.MordhauEquipment|SetbAllowFire _array_element false))))